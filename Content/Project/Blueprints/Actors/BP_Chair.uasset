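; BP_Chair is a chair actor that blows itself up when play begins.
; BeginPlay applies an upward impulse to its Geometry Collection, then after a short delay spawns a scaled explosion particle at the chair.
; It then activates the first Niagara actors tagged "flames" and "explosion" found in the level and plays an explosion sound at its location.
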(event EventBeginPlay
  (Physics|AddImpulse (Variables|Default|GetGeometryCollectionComponent) "0.000000,0.000000,50000.000000" "None" false)
  (Utilities|FlowControl|Delay 0.32)
  (Effects|SpawnEmitteratLocation "/Game/StarterContent/Particles/P_Explosion.P_Explosion" (Transformation|GetActorLocation) "0, 0, 0" "3.000000,3.000000,3.000000")
  (Utilities|FlowControl|Sequence
    (:then_0
      (bind _outactors (Actor|GetAllActorswithTag "flames"))
      (bind _asniagara_actor (Utilities|Casting|CastToNiagaraActor (Utilities|Array|Get(acopy) _outactors)))
      (Components|Activation|SetActive (Variables|/Script/Niagara.NiagaraActor|GetNiagaraComponent _asniagara_actor) true false))
    (:then_1
      (bind _outactors_2 (Actor|GetAllActorswithTag "explosion"))
      (bind _asniagara_actor_2 (Utilities|Casting|CastToNiagaraActor (Utilities|Array|Get(acopy) _outactors_2)))
      (Components|Activation|SetActive (Variables|/Script/Niagara.NiagaraActor|GetNiagaraComponent _asniagara_actor_2) true false))
    (:then_2
      (Audio|PlaySoundatLocation "/Game/StarterContent/Audio/Explosion01.Explosion01" (Transformation|GetActorLocation) "0, 0, 0" 1.0 1.0 0.0 0 0 0 0))))

(fn ConstructionScript)